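; Player hero character Blueprint that handles movement, camera look, jumping, attacking and death.
; Axis inputs drive camera-relative movement and controller yaw and pitch.
; Jump, landing and Attack set flags on Lutin_AnimBP, with the attack flag cleared after a short delay; Attack contains no hit logic.
; GameOver runs once, enabling mesh physics, disabling input and showing the GameOver widget with a UI-only cursor.
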(event `InputAxis|MoveForward`
  (params (AxisValue :type "Float (single-precision)"))
  ;[1 1 1] déplacement joueur
  (`self.AddMovementInput` (`SceneComponent.GetForwardVector` (`self.Camera`)) AxisValue))

(event `InputAction|Jump`
  (params (Key :type "Key Structure"))
  ;[1 1 1] saut joueur
  (:`Pressed`
    (`self.Jump`)
    (bind _aslutin_anim_bp (cast `/Game/Hero/animation/Lutin_AnimBP` (`SkeletalMeshComponent.GetAnimInstance` (`self.Mesh`))))
    (set `/Game/Hero/animation/Lutin_AnimBP.Jump?` true _aslutin_anim_bp)))

(event `InputAxis|MoveRight`
  (params (AxisValue :type "Float (single-precision)"))
  ;[1 1 1] déplacement joueur
  (`self.AddMovementInput` (`SceneComponent.GetRightVector` (`self.Camera`)) AxisValue))

(event `InputAxis|Turn`
  (params (AxisValue :type "Float (single-precision)"))
  ;[1 1 1] orientation de la caméra
  (`self.AddControllerYawInput` AxisValue))

(event `self.OnLanded`
  (params (Hit :type "HitResult Structure (by ref)"))
  (bind _aslutin_anim_bp (cast `/Game/Hero/animation/Lutin_AnimBP` (`SkeletalMeshComponent.GetAnimInstance` (`self.Mesh`))))
  (set `/Game/Hero/animation/Lutin_AnimBP.Jump?` false _aslutin_anim_bp))

(event `InputAxis|LookUp`
  (params (AxisValue :type "Float (single-precision)"))
  ;[1 1 1] orientation de la caméra
  (`self.AddControllerPitchInput` AxisValue))

(event `GameOver`
  (bind _returnvalue (`GameplayStatics.GetPlayerController` 0))
  ;[1 1 1] Game Over
  (`/Engine/EditorBlueprintResources/StandardMacros.DoOnce` false
    (:`Completed`
      (`PrimitiveComponent.SetSimulatePhysics` (`self.Mesh`) true)
      (`self.DisableInput` (`GameplayStatics.GetPlayerController` 0))
      (bind _returnvalue_2 (`|CreateWidget` "/Game/Widgets/GameOver.GameOver_C"))
      (`UserWidget.AddToViewport` _returnvalue_2 0)
      (set `PlayerController.bShowMouseCursor` true _returnvalue)
      (`WidgetBlueprintLibrary.SetInputMode_UIOnlyEx` _returnvalue _returnvalue_2))))

(event `InputAction|Attack`
  (params (Key :type "Key Structure"))
  (:`Pressed`
    (bind _aslutin_anim_bp (cast `/Game/Hero/animation/Lutin_AnimBP` (`SkeletalMeshComponent.GetAnimInstance` (`self.Mesh`))))
    (set `/Game/Hero/animation/Lutin_AnimBP.Attaquer` true _aslutin_anim_bp)
    (`KismetSystemLibrary.Delay` 0.5)
    (set `/Game/Hero/animation/Lutin_AnimBP.Attaquer` false _aslutin_anim_bp)))

(fn `UserConstructionScript`)