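; Lamp Blueprint that raises its point light's intensity when play begins.
; BeginPlay runs a while loop that increments the intensity in unit steps up to a fixed threshold, with no delay, so the increase completes within one frame rather than as a visible fade.
; A helper function, GetLightIntensity, returns a French text string reporting a given light's intensity, and the construction script is empty.
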(event `self.ReceiveBeginPlay`
  (bind _pointlight (`self.PointLight`))
  (while (< (`LightComponentBase.Intensity` (`self.PointLight`)) 4000.0)
    (`LightComponent.SetIntensity` _pointlight (+ (`LightComponentBase.Intensity` _pointlight) 1.0))))

(fn `GetLightIntensity`
  (params (Light :type "LightComponent Object Reference"))
  (returns (reponse :type String))
  (return (`KismetStringLibrary.Concat_StrStr` "l'intensité est de " (`KismetStringLibrary.Conv_DoubleToString` (`LightComponentBase.Intensity` Light)))))

(fn `UserConstructionScript`)