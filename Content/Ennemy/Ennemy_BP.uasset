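; Enemy Blueprint that detects the hero through a box overlap, then chases and attacks them.
; FollowHero loops on AIMoveTo, attacking on success and retrying after a short delay whether the move succeeds or fails.
; Each attack removes one clamped point from the hero's Vie (health); at zero, Tuer calls the hero's GameOver through a DoOnce.
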(event `self.Box.OnComponentBeginOverlap`
  (params (OverlappedComponent :type "PrimitiveComponent Object Reference") (OtherActor :type "Actor Object Reference") (OtherComp :type "PrimitiveComponent Object Reference") (OtherBodyIndex :type Integer) (bFromSweep :type Boolean) (SweepResult :type "HitResult Structure (by ref)"))
  ;[1 1 1] Detection du hero
  (bind _ashero_bp (cast `/Game/Hero/Hero_BP` OtherActor))
  (set `self.Hero` _ashero_bp)
  (`self.FollowHero`))

(event `FollowHero`
  ;[1 1 1] Suivre le joueur
  (`|AIMoveTo` self (0.0 0.0 0.0) (`self.Hero`)
    (:`OnSuccess`
      (`self.Attack`)
      (`KismetSystemLibrary.Delay` 1.0)
      (`self.FollowHero`))
    (:`OnFail`
      (`KismetSystemLibrary.Delay` 0.2)
      (`self.FollowHero`))))

(event `Attack`
  (bind _hero (`self.Hero`))
  (bind _output_get (set `/Game/Hero/Hero_BP.Vie` (`KismetMathLibrary.Clamp` (- (`/Game/Hero/Hero_BP.Vie` _hero) 1) 0 5) _hero))
  (if (== _output_get 0)
    (`self.Tuer`)))

(event `Tuer`
  (`/Engine/EditorBlueprintResources/StandardMacros.DoOnce` false
    (:`Completed`
      (`/Game/Hero/Hero_BP.GameOver` (`self.Hero`)))))

(fn `UserConstructionScript`)